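; BP_Enemy is an enemy NPC that chases and damages the player once it senses a pawn.
; PawnSensing's OnSeePawn sets IsSeeingPlayer and calls FollowPlayer, which uses AIMoveTo toward the first player character.
; A successful move applies damage, then waits briefly before setting CanAttack and drawing it as debug text.
; CanAttack never gates the attack, and IsSeeingPlayer is never cleared.
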(event `self.PawnSensing.OnSeePawn`
  (params (Pawn :type "Pawn Object Reference"))
  (set `self.isSeeingPlayer` true)
  (`self.FollowPlayer`))

(event `FollowPlayer`
  (set `self.canAttack` true)
  (if (`self.isSeeingPlayer`)
    (`|AIMoveTo` self (0.0 0.0 0.0) (`GameplayStatics.GetPlayerCharacter` 0) 70.0
      (:`OnSuccess`
        (`GameplayStatics.ApplyDamage` (`GameplayStatics.GetPlayerCharacter` 0) 1.25 null self)
        (`KismetSystemLibrary.Delay` 1.0)
        (bind _output_get (set `self.canAttack` true))
        (`KismetSystemLibrary.DrawDebugString` (0.0 0.0 0.0) (`KismetStringLibrary.Conv_BoolToString` _output_get) null (struct :`R` 1.0 :`G` 1.0 :`B` 1.0 :`A` 1.0) 1.0)))))

(fn `UserConstructionScript`)